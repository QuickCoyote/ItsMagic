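; BPC_MusicModifier is an actor component that scales its owner in response to a chosen audio frequency, apparently for music-reactive visuals.
; It stores the owner's original scale at BeginPlay.
; Each tick it looks up BP_EQModifier, reads that frequency's value and divides it by Dampener.
; The result becomes the scale on each enabled axis, clamped between the original scale and a fixed maximum.
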(event `self.ReceiveBeginPlay`
  (bind (_returnvalue_location _returnvalue_rotation _returnvalue_scale) (`KismetMathLibrary.BreakTransform` (`Actor.GetTransform` (`self.GetOwner`))))
  (set `self.OriginalScale` _returnvalue_scale))

(event `self.ReceiveTick`
  (params (DeltaSeconds :type "Float (single-precision)"))
  (bind _returnvalue (`self.GetOwner`))
  (bind (_originalscale_x _originalscale_y _originalscale_z) (`KismetMathLibrary.BreakVector` (`self.OriginalScale`)))
  (bind _frequencyvalue (`self.FrequencyValue`))
  (bind (_returnvalue_x _returnvalue_y _returnvalue_z) (`KismetMathLibrary.BreakVector` (`Actor.GetActorScale3D` _returnvalue)))
  (bind _returnvalue_2 (`GameplayStatics.GetActorOfClass` "/Game/Blueprints/BP_EQModifier.BP_EQModifier_C"))
  (bind _value (`/Game/Blueprints/BP_EQModifier.GetFrequencyValue` _returnvalue_2 (`self.Frequency`)))
  (set `self.FrequencyValue` (/ _value (`self.Dampener`)))
  (`|ExecutionSequence`
    (:`then_0`
      (if (`self.ScaleX`)
        (`Actor.SetActorScale3D` _returnvalue (`KismetMathLibrary.MakeVector` (`KismetMathLibrary.FClamp` _frequencyvalue _originalscale_x 500.0) _returnvalue_y _returnvalue_z))))
    (:`then_1`
      (if (`self.ScaleY`)
        (`Actor.SetActorScale3D` _returnvalue (`KismetMathLibrary.MakeVector` _returnvalue_x (`KismetMathLibrary.FClamp` _frequencyvalue _originalscale_y 500.0) _returnvalue_z))))
    (:`then_2`
      (if (`self.ScaleZ`)
        (`Actor.SetActorScale3D` _returnvalue (`KismetMathLibrary.MakeVector` _returnvalue_x _returnvalue_y (`KismetMathLibrary.FClamp` _frequencyvalue _originalscale_z 500.0)))))))