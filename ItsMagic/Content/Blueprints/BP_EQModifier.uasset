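; Music equalizer actor that plays a song and animates a row of bar actors to its frequency spectrum.
; BeginPlay gathers the bars into an X-ordered array and starts the audio.
; Each Tick samples a short spectrum window slightly behind game time and sets each bar's Z scale through ScaleBars' clamped cubic curve.
; GetFrequencyValue returns a single band on request; the song-end check is unconnected.
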(event `self.ReceiveBeginPlay`
  (bind _returnvalue_x (`KismetMathLibrary.BreakVector` (`self.K2_GetActorLocation`)))
  (bind (_eq_bars _eq_bars_2) (`self.EQ-Bars`))
  (bind _audio (`self.Audio`))
  (bind _outactors (`GameplayStatics.GetAllActorsOfClass` null))
  (for _array_element _outactors
    (for (_ _array_index) _eq_bars_2
      (bind _returnvalue_x_2 (`KismetMathLibrary.BreakVector` (`self.K2_GetActorLocation` _array_element)))
      (if (not (< _returnvalue_x _returnvalue_x_2))
        (break)))
    (`KismetArrayLibrary.Array_Insert` _eq_bars_2 _array_element _array_index)
    (`AudioComponent.SetSound` _audio (`self.Song`))
    (`AudioComponent.Play` _audio -2.0)
    (set `self.IsPlaying` true)))

(event `self.ReceiveTick`
  (params (DeltaSeconds :type "Float (single-precision)"))
  (bind _frequencies (`self.Frequencies`))
  (for (_array_element _array_index) _frequencies
    (if (> (`|GetArrayItem` _frequencies _array_index) 0.0)
      (set `self.FrequencyTotal` (+ _array_element (`self.FrequencyTotal`)))))
  (set `self.FrequencyTotal` 0.0)
  (bind _outspectrum (`self.CalculateFrequencySpectrum` (`self.Song`) 0 (+ (`KismetSystemLibrary.GetGameTimeInSeconds`) -0.3) 0.1 (`self.Spectrum Width`)))
  (set `self.Frequencies` _outspectrum)
  (for (_array_element_2 _array_index_2) (`.EQ-Bars` (`self.EQ-Bars`))
    (`self.SetActorScale3D` _array_element_2 (`KismetMathLibrary.MakeVector` 1.0 1.0 (`self.ScaleBars` (`|GetArrayItem` (`self.Frequencies`) _array_index_2))))))

(fn `GetFrequencyValue`
  (params (Frequency :type Integer))
  (returns (Value :type "Float (double-precision)"))
  (bind _outspectrum (`self.CalculateFrequencySpectrum` (`self.Song`) 0 (+ (`KismetSystemLibrary.GetGameTimeInSeconds`) -0.3) 0.17 (`self.Spectrum Width`)))
  (return (`|GetArrayItem` _outspectrum (`KismetMathLibrary.Clamp` Frequency 0 (`self.Spectrum Width`)))))

(fn `ScaleBars`
  (params (A :type "Float (double-precision)"))
  (returns (ReturnValue :type "Float (double-precision)"))
  (bind _returnvalue (`KismetMathLibrary.FClamp` (/ A 15.0) 0.0 2.75))
  (return (+ (* _returnvalue _returnvalue _returnvalue) 0.1)))

(fn `UserConstructionScript`)