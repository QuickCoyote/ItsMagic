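; BPC_MusicModifier is a Blueprint that scales an actor with the music frequency value read from BP_EQModifier.
; Every Tick it looks up that actor by class and requests the value for its Frequency setting.
; ScaleX, ScaleY and ScaleZ flags choose the axis.
; Each write zeroes the other two axes, so the last enabled flag wins instead of combining.
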(event `self.ReceiveTick`
  (params (DeltaSeconds :type "Float (single-precision)"))
  (bind _frequencyvalue (`self.FrequencyValue`))
  (bind _returnvalue (`GameplayStatics.GetActorOfClass` "/Game/Blueprints/BP_EQModifier.BP_EQModifier_C"))
  (`/Game/Blueprints/BP_EQModifier.GetFrequencyValue` _returnvalue (`self.Frequency`))
  (`|ExecutionSequence`
    (:`then_0`
      (if (`self.ScaleX`)
        (`Actor.SetActorScale3D` (`KismetMathLibrary.MakeVector` _frequencyvalue))))
    (:`then_1`
      (if (`self.ScaleY`)
        (`Actor.SetActorScale3D` (`KismetMathLibrary.MakeVector` 0.0 _frequencyvalue))))
    (:`then_2`
      (if (`self.ScaleZ`)
        (`Actor.SetActorScale3D` (`KismetMathLibrary.MakeVector` 0.0 0.0 _frequencyvalue))))))